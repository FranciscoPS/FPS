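; MyCharacterBP is an FPS player character that handles movement, look input, HUD creation and weapon equipping.
; Movement follows control yaw only, while look axes feed controller pitch and yaw.
; BeginPlay adds the HUD widget to the viewport and equips the base weapon.
; EquipWeapon stores the class, swaps it into the Weapon child actor component and initializes the spawned actor through the PlayerWeaponI interface.
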(event Custom|EquipWeapon
  (params (Weapon :type Player%20Base%20Weapon%20BP%20Class%20Reference))
  (bind _childactor (Variables|/Script/Engine.ChildActorComponent|GetChildActor (Variables|Default|GetWeapon)))
  (bind _output_get (Variables|Default|SetCurrentWeapon Weapon))
  (ChildActorComponent|SetChildActorClass (Variables|Default|GetWeapon) _output_get)
  (if (Utilities|DoesObjectImplementInterface _childactor "/Game/FPS/Blueprint/PlayerWeaponI.PlayerWeaponI_C")
    (Class|PlayerWeaponI|InitializeWeapon(Message) _childactor)))

(event EventBeginPlay
  (|CallParentFunction)
  (bind _returnvalue (UserInterface|CreateWidget "/Game/FPS/Blueprint/HUD/HUDWidtget_BP.HUDWidtget_BP_C"))
  (UserInterface|Viewport|AddtoViewport _returnvalue 0)
  (CallFunction|EquipWeapon "/Game/FPS/Blueprint/Player/PlayerBaseWeapon_BP.PlayerBaseWeapon_BP_C"))

(event Collision|EventActorBeginOverlap
  (params (OtherActor :type Actor%20Object%20Reference)))

(event EventTick
  (params (DeltaSeconds :type Float%20%28single-precision%29)))

(event Input|AxisEvents|InputAxisLookVertical
  (params (AxisValue :type Float%20%28single-precision%29))
  (Pawn|Input|AddControllerPitchInput AxisValue))

(event Input|AxisEvents|InputAxisLookHorizontal
  (params (AxisValue :type Float%20%28single-precision%29))
  (Pawn|Input|AddControllerYawInput AxisValue))

(event Input|AxisEvents|InputAxismoveForward
  (params (AxisValue :type Float%20%28single-precision%29))
  (Pawn|Input|AddMovementInput (Math|Vector|GetForwardVector (Math|Rotator|MakeRotator 0.0 0.0 (.yaw (Pawn|GetControlRotation :!class /Script/Engine.Pawn)))) AxisValue false))

(event Input|AxisEvents|InputAxismoveRight
  (params (AxisValue :type Float%20%28single-precision%29))
  (Pawn|Input|AddMovementInput (Math|Vector|GetRightVector (Math|Rotator|MakeRotator 0.0 0.0 (.yaw (Pawn|GetControlRotation :!class /Script/Engine.Pawn)))) AxisValue false))

(fn ConstructionScript)