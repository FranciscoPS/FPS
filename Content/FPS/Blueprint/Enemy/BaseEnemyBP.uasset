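; Base enemy for the FPS, drawn as an eight-direction billboard sprite and driven by a behavior tree started on its AI controller.
; Each tick the Paper2D flipbook yaws toward the player camera.
; Unless dead or paused, it then derives the horizontal angle and side between its facing and the player using dot products.
; That sector and whether velocity is non-zero select the directional walk or idle flipbook.
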(event EventBeginPlay
  (|CallParentFunction)
  (bind _asenemy_controller_ai_bp (Utilities|Casting|CastToEnemyControllerAI_BP (Pawn|GetController)))
  (AI|RunBehaviorTree _asenemy_controller_ai_bp (Variables|Default|GetBehaviourTree)))

(event Collision|EventActorBeginOverlap
  (params (OtherActor :type Actor%20Object%20Reference))
  (|CallParentFunction OtherActor) ; This node is disabled and will not be called.\nDrag off pins to build functionality.
)

(event EventTick
  (params (DeltaSeconds :type Float%20%28single-precision%29))
  (|CallParentFunction DeltaSeconds)
  (Utilities|SpriteFacePlayer
    (:Out
      (if (not (or (Variables|Default|GetIsDead) (Variables|Default|GetPauseAngleCalculation)))
        (Utilities|GetEnemyAngle
          (:Out
            (Utilities|CheckifWalking
              (:Out
                (Utilities|CalculateFlip)))))))))

(fn ConstructionScript
  (|CallParentFunction))

(fn SetFlipbook
  (params (Walk :type Paper%20Flipbook%20Object%20Reference) (idle :type Paper%20Flipbook%20Object%20Reference))
  (bind _paperflipbook (Variables|Default|GetPaperFlipbook))
  (if (Variables|Default|GetIsWalking)
    (Sprite|SetFlipbook _paperflipbook Walk)
    (else
      (Sprite|SetFlipbook _paperflipbook idle))))