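; Base enemy character for an FPS, drawn as a Paper2D flipbook billboard with Doom-style eight-direction sprites.
; It runs a behavior tree on its AI controller and yaws the sprite toward the camera every tick.
; The enemy's angle and side relative to the player, plus velocity, select walk or idle flipbooks.
; Damage and death pause that selection for their animations; death also stops AI and capsule collision, while attack events remain stubs.
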(event Custom|melleAttack)

(event Custom|rangeattack
  (Development|PrintString "attacking"))

(event EventBeginPlay
  (|CallParentFunction)
  (bind _asenemy_aicontroller (Utilities|Casting|CastToEnemyAIController (Pawn|GetController)))
  (AI|RunBehaviorTree _asenemy_aicontroller (Variables|Default|GetBHTree)))

(event Collision|EventActorBeginOverlap
  (params (OtherActor :type Actor%20Object%20Reference))
  (|CallParentFunction OtherActor) ; This node is disabled and will not be called.\nDrag off pins to build functionality.
)

(event EventTick
  (params (DeltaSeconds :type Float%20%28single-precision%29))
  (|CallParentFunction DeltaSeconds)
  (Utilities|SpriteFacePlayer
    (:Out
      (if (not (or (Variables|Default|GetisDead) (Variables|Default|GetPauseAngleCalculations)))
        (Utilities|GetEnemyAngle
          (:Out
            (Utilities|CheckifWalking
              (:out
                (Utilities|CalculateFlip)))))))))

(event EventKillCharacter
  (bind _paperflipbook (Variables|Default|GetPaperFlipbook))
  (|CallParentFunction)
  (bind _asenemy_aicontroller (Utilities|Casting|CastToEnemyAIController (Pawn|GetController)))
  (AI|Logic|StopLogic (Variables|/Script/AIModule.AIController|GetBrainComponent _asenemy_aicontroller) "")
  (Variables|Default|SetisDead true)
  (Collision|SetCollisionEnabled (Variables|Default|GetCapsuleComponent) "NoCollision")
  (Sprite|SetFlipbook _paperflipbook (Variables|Default|Getdiying))
  (Utilities|FlowControl|Delay (Class|PaperFlipbookComponent|GetFlipbookLength _paperflipbook))
  (Sprite|SetFlipbook (Variables|Default|GetPaperFlipbook) (Variables|Default|Getdead)))

(event EventTakeDamage
  (params (Data :type Gameplay%20Cue%20Parameters%20Structure))
  (bind _paperflipbook (Variables|Default|GetPaperFlipbook))
  (|CallParentFunction Data)
  (if (not (Variables|Default|GetisDead))
    (Variables|Default|SetPauseAngleCalculations true)
    (Sprite|SetFlipbook _paperflipbook (Variables|Default|GetDamaged))
    (Utilities|FlowControl|Delay (Class|PaperFlipbookComponent|GetFlipbookLength _paperflipbook))
    (Variables|Default|SetPauseAngleCalculations false)))

(fn ConstructionScript
  (|CallParentFunction))

(fn SetFlipbook
  (params (Walk :type Paper%20Flipbook%20Object%20Reference) (Iddle :type Paper%20Flipbook%20Object%20Reference))
  (bind _paperflipbook (Variables|Default|GetPaperFlipbook))
  (if (Variables|Default|GetIsWalking)
    (Sprite|SetFlipbook _paperflipbook Walk)
    (else
      (Sprite|SetFlipbook _paperflipbook Iddle))))