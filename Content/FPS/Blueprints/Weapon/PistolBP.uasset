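; Pistol weapon Blueprint that displays idle and shooting animations as Paper2D flipbooks.
; InitializeWeapon shows the idle flipbook and caches the player pawn as MyPlayerBP.
; ShootWeapon calls the player's UI update, plays the shoot flipbook, then returns to idle after a delay matching that flipbook's length.
; It contains no hit, damage or ammo logic, and the default BeginPlay, overlap and Tick events are disabled.
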(event Custom|ShootWeapon
  (bind _paperflipbook (Variables|Default|GetPaperFlipbook))
  (Default|UpdateUI (Variables|Default|Getplayer))
  ;[0.15 0.15 0.15 0.5] ShootAnim
  (Sprite|SetFlipbook _paperflipbook (Variables|Default|GetShootFlipbook))
  (Utilities|FlowControl|Delay (Class|PaperFlipbookComponent|GetFlipbookLength _paperflipbook))
  (Sprite|SetFlipbook (Variables|Default|GetPaperFlipbook) (Variables|Default|GetIdleFlipBook)))

(event EventBeginPlay
  (|CallParentFunction) ; This node is disabled and will not be called.\nDrag off pins to build functionality.
)

(event Collision|EventActorBeginOverlap
  (params (OtherActor :type Actor%20Object%20Reference))
  (|CallParentFunction OtherActor) ; This node is disabled and will not be called.\nDrag off pins to build functionality.
)

(event EventTick
  (params (DeltaSeconds :type Float%20%28single-precision%29))
  (|CallParentFunction DeltaSeconds) ; This node is disabled and will not be called.\nDrag off pins to build functionality.
)

(event EventInitializeWeapon
  ;[0.15 0.15 0.15 0.5] EquipWeapon
  (Sprite|SetFlipbook (Variables|Default|GetPaperFlipbook) (Variables|Default|GetIdleFlipBook))
  (Development|SetHiddeninGame (Variables|Default|GetPaperFlipbook) false false)
  (bind _asmy_player_bp (Utilities|Casting|CastToMyPlayerBP (Game|Player|GetPlayerPawn 0)))
  (Variables|Default|Setplayer _asmy_player_bp))

(fn ConstructionScript
  (|CallParentFunction))