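; Stat pickup for an FPS that represents either health or armor, in a small or large size.
; The Construction Script runs SetStatPickUp, which sets the sprite's color by type, its scale by size, and the matching pickup gameplay tag.
; FullHealthCheck and FullArmorCheck read an Ability System attribute, adding a Player Full tag to the pickup's tags at 100 and removing it otherwise.
; The event graph is inactive, and neither check is called here.
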(event EventBeginPlay
  (|CallParentFunction) ; This node is disabled and will not be called.\nDrag off pins to build functionality.
)

(event Collision|EventActorBeginOverlap
  (params (OtherActor :type Actor%20Object%20Reference)))

(event EventTick
  (params (DeltaSeconds :type Float%20%28single-precision%29))
  (|CallParentFunction DeltaSeconds) ; This node is disabled and will not be called.\nDrag off pins to build functionality.
)

(fn ConstructionScript
  (|CallParentFunction)
  (CallFunction|SetStatPickUp))

(fn SetStatPickUp
  (bind _papersprite (Variables|Default|GetPaperSprite))
  (bind _pickup_size (Variables|Default|GetPickup%20Size))
  (bind _papersprite_2 (Variables|Default|GetPaperSprite))
  (switch Utilities|FlowControl|Switch|SwitchonPickupTypeEnum (Variables|Default|GetPickup%20Type)
    (:NewEnumerator0
      (Sprite|SetSpriteColor _papersprite "(R=0.187288,G=0.533067,B=1.000000,A=1.000000)")
      (switch Utilities|FlowControl|Switch|SwitchonPickUpSizeEnum _pickup_size
        (:NewEnumerator0
          (Transformation|SetRelativeScale3D _papersprite_2 "2.000000,2.000000,2.000000")
          (Variables|Default|SetPickUpTag "(GameplayTags=((TagName=\"Pickup.Armor.Small\")))"))
        (:NewEnumerator1
          (Transformation|SetRelativeScale3D _papersprite_2 "4.000000,4.000000,4.000000")
          (Variables|Default|SetPickUpTag "(GameplayTags=((TagName=\"Pickup.Armor.Large\")))"))))
    (:NewEnumerator1
      (Sprite|SetSpriteColor _papersprite "(R=1.000000,G=0.159491,B=0.149941,A=1.000000)")
      (switch Utilities|FlowControl|Switch|SwitchonPickUpSizeEnum _pickup_size
        (:NewEnumerator0
          (Transformation|SetRelativeScale3D _papersprite_2 "2.000000,2.000000,2.000000")
          (Variables|Default|SetPickUpTag "(GameplayTags=((TagName=\"Pickup.Health.Small\")))"))
        (:NewEnumerator1
          (Transformation|SetRelativeScale3D _papersprite_2 "4.000000,4.000000,4.000000")
          (Variables|Default|SetPickUpTag "(GameplayTags=((TagName=\"Pickup.Health.Large\")))"))))))

(fn FullHealthCheck
  (params (AbilitySystem :type Ability%20System%20Component%20Object%20Reference))
  (bind _pickuptag (Variables|Default|GetPickUpTag))
  (if (== (.ReturnValue (Ability|Attribute|GetFloatAttributefromAbilitySystemComponent AbilitySystem "(AttributeName=\"Health\",Attribute=/Script/FPS.FPSAttributeSet:Health,AttributeOwner=\"/Script/CoreUObject.Class'/Script/FPS.FPSAttributeSet'\")")) 1e+02)
    (GameplayTags|AddGameplayTag _pickuptag "(TagName=\"Player.Health.Full\")" :!class /Script/GameplayTags.BlueprintGameplayTagLibrary)
    (else
      (GameplayTags|RemoveGameplayTag _pickuptag "(TagName=\"Player.Health.Full\")" :!class /Script/GameplayTags.BlueprintGameplayTagLibrary))))

(fn FullArmorCheck
  (params (AbilitySystem :type Ability%20System%20Component%20Object%20Reference))
  (bind _pickuptag (Variables|Default|GetPickUpTag))
  (if (== (.ReturnValue (Ability|Attribute|GetFloatAttributefromAbilitySystemComponent AbilitySystem "(AttributeName=\"Armor\",Attribute=/Script/FPS.FPSAttributeSet:Armor,AttributeOwner=\"/Script/CoreUObject.Class'/Script/FPS.FPSAttributeSet'\")")) 1e+02)
    (GameplayTags|AddGameplayTag _pickuptag "(TagName=\"Player.Armor.Full\")" :!class /Script/GameplayTags.BlueprintGameplayTagLibrary)
    (else
      (GameplayTags|RemoveGameplayTag _pickuptag "(TagName=\"Player.Armor.Full\")" :!class /Script/GameplayTags.BlueprintGameplayTagLibrary))))