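; Weapon pickup actor that gives the player a weapon when overlapped.
; The construction script sets its Paper2D sprite from the WeaponToEquip enum, showing a pistol or launcher image, or nothing for None.
; On overlap it casts the other actor to MyPlayerBP, calls PickupWeapon with that weapon, then destroys itself.
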(event EventBeginPlay)

(event Collision|EventActorBeginOverlap
  (params (OtherActor :type Actor%20Object%20Reference))
  (bind _asmy_player_bp (Utilities|Casting|CastToMyPlayerBP OtherActor))
  (Default|PickupWeapon _asmy_player_bp (Variables|Weapon|GetWeaponToEquip))
  (Actor|DestroyActor))

(event EventTick
  (params (DeltaSeconds :type Float%20%28single-precision%29))
  (|CallParentFunction DeltaSeconds))

(fn ConstructionScript
  (bind _papersprite (Variables|Default|GetPaperSprite))
  (switch Utilities|FlowControl|Switch|SwitchonWeaponEnum (Variables|Weapon|GetWeaponToEquip)
    (:NewEnumerator0
      (Rendering|Components|Sprite|SetSprite _papersprite 0))
    (:NewEnumerator1
      (Rendering|Components|Sprite|SetSprite _papersprite "/Game/FPS/Sprites/pistol_pickup_Sprite.pistol_pickup_Sprite"))
    (:NewEnumerator2
      (Rendering|Components|Sprite|SetSprite _papersprite "/Game/FPS/Sprites/launcher_pickup_Sprite.launcher_pickup_Sprite"))))