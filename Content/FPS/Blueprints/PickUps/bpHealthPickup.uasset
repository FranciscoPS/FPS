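; Health pickup actor that reacts when the player pawn overlaps it, using the Gameplay Ability System.
; On overlap with MyPlayerBP it runs FullHealthCheck on the player's Ability System Component, then tries to activate abilities matching PickUpTag.
; Only a successful activation calls the player's ItemPickup and destroys the pickup.
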(event EventBeginPlay
  (|CallParentFunction) ; This node is disabled and will not be called.\nDrag off pins to build functionality.
)

(event Collision|EventActorBeginOverlap
  (params (OtherActor :type Actor%20Object%20Reference))
  (|CallParentFunction OtherActor)
  (bind _asmy_player_bp (Utilities|Casting|CastToMyPlayerBP OtherActor))
  (CallFunction|FullHealthCheck (Variables|/Script/FPS.FPSBaseCharacter|GetAbilitySystemComponent _asmy_player_bp))
  (bind _returnvalue (Abilities|TryActivateAbilitiesbyTag (Variables|/Script/FPS.FPSBaseCharacter|GetAbilitySystemComponent _asmy_player_bp) (Variables|Default|GetPickUpTag) false))
  (if _returnvalue
    (Default|ItemPickup _asmy_player_bp)
    (Actor|DestroyActor)))

(event EventTick
  (params (DeltaSeconds :type Float%20%28single-precision%29))
  (|CallParentFunction DeltaSeconds) ; This node is disabled and will not be called.\nDrag off pins to build functionality.
)

(fn ConstructionScript
  (|CallParentFunction))