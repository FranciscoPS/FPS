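; BP_Rocket is a rocket projectile shown as a Paper2D sprite that damages enemies on impact.
; Each tick, the sprite yaws to face the player camera as a billboard.
; When the projectile movement stops, a hit BaseEnemyBP receives GE_LauncherDamage through its own Gameplay Ability System component.
; An explosion actor then spawns at the impact point, aligned to the surface normal, and the rocket destroys itself.
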(event OnProjectileStop(ProjectileMovement)
  (params (ImpactResult :type Hit%20Result%20Structure%20%28by%20ref%29))
  (bind _asbase_enemy_bp (Utilities|Casting|CastToBaseEnemyBP (.hitactor ImpactResult))
    (:then
      (GameplayEffects|ApplyGameplayEffectToTarget (Variables|/Script/FPS.FPSBaseCharacter|GetAbilitySystemComponent _asbase_enemy_bp) "/Game/FPS/Blueprints/Abilities/GE_LauncherDamage.GE_LauncherDamage_C" (Variables|/Script/FPS.FPSBaseCharacter|GetAbilitySystemComponent _asbase_enemy_bp) 0.0 (GameplayEffects|MakeEffectContext (Variables|/Script/FPS.FPSBaseCharacter|GetAbilitySystemComponent _asbase_enemy_bp))))
    (:CastFailed
      _))
  (Game|SpawnActorfromClass "/Game/FPS/Blueprints/Abilities/RocketExpotionBP.RocketExpotionBP_C" (Math|Transform|MakeTransform (.impactpoint ImpactResult) (Math|Conversions|RotationFromXVector (.impactnormal ImpactResult)) "1.000000,1.000000,1.000000") "Undefined" "MultiplyWithRoot" 0 0)
  (Actor|DestroyActor))

(event EventBeginPlay)

(event Collision|EventActorBeginOverlap
  (params (OtherActor :type Actor%20Object%20Reference)))

(event EventTick
  (params (DeltaSeconds :type Float%20%28single-precision%29))
  (bind _papersprite (Variables|Default|GetPaperSprite))
  (Transformation|SetWorldRotation _papersprite (Math|Rotator|MakeRotator 0.0 0.0 (- (.yaw (Math|Rotator|FindLookatRotation (Transformation|GetWorldLocation _papersprite) (Camera|GetCameraLocation (Game|GetPlayerCameraManager 0)))) 9e+01)) false false))

(fn ConstructionScript)