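; Base Gameplay Ability for FPS weapons, with empty FireWeapon and Reset hooks for child abilities to override.
; On activation it commits, starts listening for the weapon event tag, fires, then ends after the remaining cooldown, which sets the fire rate.
; ApplyEfect sends target data to the attacker as a gameplay event, and the listener applies WeaponEffect to that target.
; Ending the ability stops both tasks and calls Reset.
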(event Custom|WaitForEvent
  ;[0.15 0.15 0.15 0.5] Wait for Gameplay Tag
  (bind (_asynctaskproxy _payload) (Ability|Tasks|WaitGameplayEvent (Variables|Default|GetWeaponEventTag) 0)
    (:then
      (Variables|Default|SetGameplayEventWaitTask _asynctaskproxy))
    (:EventReceived
      (GameplayEffects|ApplyGameplayEffectToTarget (.TargetData (Utilities|Struct|BreakGameplayEventData _payload)) (Variables|Default|GetWeaponEffect) 1 1))))

(event Custom|FireWeapon
  ;[0.15 0.15 0.15 0.5] Override
)

(event Ability|EventActivateAbility
  ;[0.15 0.15 0.15 0.5] Activation
  (Ability|CommitAbility)
  (CallFunction|WaitforEvent)
  (CallFunction|FireWeapon)
  ;[0.15 0.15 0.15 0.5] Ability Duration
  (bind _asynctaskproxy (GameplayTasks|TaskWaitDelay 0 (Class|GameplayAbility|GetCooldownTimeRemaining))
    (:then
      (Variables|Default|SetFireRateDelay _asynctaskproxy))
    (:OnFinish
      (Ability|EndAbility))))

(event Ability|EventOnEndAbility
  (params (bWasCancelled :type Boolean))
  (bind _gameplayeventwaittask (Variables|Default|GetGameplayEventWaitTask))
  (bind _fireratedelay (Variables|Default|GetFireRateDelay))
  ;[0.15 0.15 0.15 0.5] End Ability
  (Utilities|IsValid _gameplayeventwaittask
    (:Is%20Valid
      (GameplayTasks|EndTask _gameplayeventwaittask)
      (Utilities|IsValid _fireratedelay
        (:Is%20Valid
          (GameplayTasks|EndTask _fireratedelay)
          (CallFunction|Reset))))))

(fn Reset)

(fn ApplyEfect
  (params (AttacikngActor :type Actor%20Object%20Reference) (TargetActor :type Actor%20Object%20Reference))
  (Ability|SendGameplayEventtoActor AttacikngActor (Variables|Default|GetWeaponEventTag) (Utilities|Struct|MakeGameplayEventData "(TagName=\"\")" 0 TargetActor 0 0 "()" "(GameplayTags=)" "(GameplayTags=)" 0.0 (Ability|TargetData|AbilityTargetDatafromActor TargetActor))))