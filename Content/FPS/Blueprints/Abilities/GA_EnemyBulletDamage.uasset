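; Gameplay ability for the pistol enemy's hitscan shot, applying an effect to the BaseCharacterBP it hits.
; FireWeapon caches the owning PistolEnemyBP, then line-traces on Visibility from its capsule along the forward vector for WeaponRange, with persistent debug drawing.
; A valid hit actor is returned for the effect.
; Only when none is found does a pooled object spawn at the impact point, aligned to the normal.
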(event EventFireWeapon
  (CallFunction|GetEnemy)
  (bind _actor (CallFunction|GetLinetrace))
  (bind _asbase_character_bp (Utilities|Casting|CastToBaseCharacterBP _actor))
  (CallFunction|ApplyEfect (Variables|Default|GetPiostolEnemy) _asbase_character_bp))

(fn GetLinetrace
  (bind _piostolenemy (Variables|Default|GetPiostolEnemy))
  (bind _capsulecomponent (Variables|/Script/Engine.Character|GetCapsuleComponent _piostolenemy))
  (bind _returnvalue (Transformation|GetWorldLocation _capsulecomponent))
  (bind _outhit (Collision|LineTraceByChannel _returnvalue (+ _returnvalue (* (Math|Vector|GetForwardVector (Transformation|GetWorldRotation _capsulecomponent)) (Variables|Default|GetWeaponRange))) "TraceTypeQuery1" false 0 "Persistent" true "(R=0.089341,G=0.105606,B=1.000000,A=1.000000)"))
  (Utilities|IsValid (.HitActor (Collision|BreakHitResult _outhit))
    (:Is%20Valid
      (return (.HitActor (Collision|BreakHitResult _outhit))))
    (:Is%20Not%20Valid
      (bind _returnvalue_2 (Class|ObjectPooling|SpawnPooledObject (Variables|/Game/FPS/Blueprints/Enemy/PistolEnemyBP.PistolEnemyBP_C|GetObjectPooling (Variables|Default|GetPiostolEnemy))))
      (Transformation|SetActorLocation _returnvalue_2 (.ImpactPoint (Collision|BreakHitResult _outhit)) false false)
      (Transformation|SetActorRotation _returnvalue_2 (Math|Conversions|RotationFromXVector (.Normal (Collision|BreakHitResult _outhit)))))))

(fn GetEnemy
  (Utilities|IsValid (Variables|Default|GetPiostolEnemy)
    (:Is%20Valid
      _)
    (:Is%20Not%20Valid
      (bind _aspistol_enemy_bp (Utilities|Casting|CastToPistolEnemyBP (.owneractor (Ability|GetActorInfo))))
      (Variables|Default|SetPiostolEnemy _aspistol_enemy_bp)))
  (return))