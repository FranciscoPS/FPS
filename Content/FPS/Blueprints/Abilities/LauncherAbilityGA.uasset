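; Gameplay ability that fires the player's rocket launcher in the FPS game.
; FireWeapon checks that an ability-system attribute is positive, applies the rocket-spend effect, then calls ShootWeapon on the launcher child actor.
; Helper functions lazily cache the player and launcher references.
; An uncalled LineTrace helper traces from the camera with persistent debug drawing, returning the hit actor or otherwise placing a pooled object at the impact point.
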(event EventFireWeapon
  (bind _launcherpistolcomponent (Variables|Default|GetLauncherPistolComponent))
  ;[0.15 0.15 0.15 0.5] fire pistol
  (CallFunction|GetPlayer)
  (if (> (.ReturnValue (Ability|Attribute|GetFloatAttributefromAbilitySystemComponent (Variables|/Script/FPS.FPSBaseCharacter|GetAbilitySystemComponent (Variables|Default|GetPlayer)) "(AttributeName=\"Rockets\",Attribute=/Script/FPS.FPSAttributeSet:Rockets,AttributeOwner=\"/Script/CoreUObject.Class'/Script/FPS.FPSAttributeSet'\")")) 0.0)
    (CallFunction|GetWeapon)
    (Utilities|IsValid _launcherpistolcomponent
      (:Is%20Valid
        (Ability|ApplyGameplayEffectToOwner "/Game/FPS/Blueprints/Abilities/GEplayerRocketSpend.GEplayerRocketSpend_C")
        (Default|ShootWeapon _launcherpistolcomponent)))))

(fn GetPlayer
  (Utilities|IsValid (Variables|Default|GetPlayer)
    (:Is%20Valid
      _)
    (:Is%20Not%20Valid
      (bind _asmy_player_bp (Utilities|Casting|CastToMyPlayerBP (.owneractor (Ability|GetActorInfo))))
      (Variables|Default|SetPlayer _asmy_player_bp)))
  (return))

(fn GetWeapon
  (Utilities|IsValid (Variables|Default|GetLauncherPistolComponent)
    (:Is%20Valid
      _)
    (:Is%20Not%20Valid
      (bind _aslauncher_bp (Utilities|Casting|CastToLauncherBP (Variables|/Script/Engine.ChildActorComponent|GetChildActor (Variables|/Game/FPS/Blueprints/Player/MyPlayerBP.MyPlayerBP_C|GetWeapon (Variables|Default|GetPlayer)))))
      (Variables|Default|SetLauncherPistolComponent _aslauncher_bp)))
  (return))

(fn LineTrace
  (bind _player (Variables|Default|GetPlayer))
  (bind _camera (Variables|/Game/FPS/Blueprints/Player/MyPlayerBP.MyPlayerBP_C|GetCamera _player))
  (bind _returnvalue (Transformation|GetWorldLocation _camera))
  (bind _outhit (Collision|LineTraceByChannel _returnvalue (+ _returnvalue (* (Math|Vector|GetForwardVector (Transformation|GetWorldRotation _camera)) (Variables|Default|GetWeaponRange))) "TraceTypeQuery1" false 0 "Persistent"))
  (Utilities|IsValid (.HitActor (Collision|BreakHitResult _outhit))
    (:Is%20Valid
      (return (.HitActor (Collision|BreakHitResult _outhit))))
    (:Is%20Not%20Valid
      (bind _returnvalue_2 (Class|ObjectPooling|SpawnPooledObject (Variables|/Game/FPS/Blueprints/Player/MyPlayerBP.MyPlayerBP_C|GetObjectPooling (Variables|Default|GetPlayer))))
      (Transformation|SetActorLocation _returnvalue_2 (.ImpactPoint (Collision|BreakHitResult _outhit)) false false)
      (Transformation|SetActorRotation _returnvalue_2 (Math|Conversions|RotationFromXVector (.Normal (Collision|BreakHitResult _outhit)))))))