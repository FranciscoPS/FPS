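; Player character Blueprint for an FPS, handling movement, look, weapon pickup and switching, firing, and HUD updates.
; Weapons come from a data table, join an owned list, and equip through a child actor initialized via an interface, setting the fire tag.
; Firing and ammo pickups activate Gameplay Ability System abilities by tag, with ammo capped at maximums.
; UpdateUI pushes attribute values to the HUD, while timelines flash it on damage and pickups.
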(event Custom|EquipWeapon
  (params (newWeapon :type ST%20Weapon%20Data%20Structure))
  ;[0.15 0.15 0.15 0.5] Equip Weapon
  (bind _output_get (Variables|Player|SetCurrentWeapon newWeapon))
  (bind _weaponactor (CallFunction|InitWeapon (.weapon _output_get)))
  (Default|Switchhweapon (Variables|Default|GetHUD) (.weaponname (Variables|Player|GetCurrentWeapon)))
  (CallFunction|UpdateUI)
  (switch Utilities|FlowControl|Switch|SwitchonWeaponEnum (.weaponname (Variables|Player|GetCurrentWeapon))
    (:NewEnumerator0
      (Variables|Default|SetweaponFireTag ""))
    (:NewEnumerator1
      (Variables|Default|SetweaponFireTag "(GameplayTags=((TagName=\"Player.Pistol.Fire\")))"))
    (:NewEnumerator2
      (Variables|Default|SetweaponFireTag "(GameplayTags=((TagName=\"Player.launcher.fire\")))"))))

(event Custom|ItemPickup
  ;[0.15 0.15 0.15 0.5] itemPickup
  (CallFunction|UpdateUI)
  (bind _alpha (Timeline|PickUpFlash PlayFromStart)
    (:Update
      (Default|SetFlashColor (Variables|Default|GetHUD) "(R=0.345401,G=0.393605,B=1.000000,A=1.000000)" _alpha))))

(event Custom|pickupWeapon
  (params (weapon :type WeaponEnum%20Enum :default "NewEnumerator0"))
  ;[0.15 0.15 0.15 0.5] WeaponPickupData
  (bind (_weapondata _weaponfound) (CallFunction|GetWeaponfromData weapon))
  (if _weaponfound
    (bind _output_get (Variables|Default|SetweaponToPickup _weapondata))
    (if (CallFunction|HasWeapon (.weaponName (Utilities|Struct|BreakSTWeaponData _output_get)))
      (CallFunction|AddAmmo (.amoType (Utilities|Struct|BreakSTWeaponData _output_get)) (.ammosize (Utilities|Struct|BreakSTWeaponData _output_get)))
      (else
        (CallFunction|AddWeapon)))
    (else
      (Development|PrintString "ERRORWeaponDoesNotExist"))))

(event Custom|add%20ammo
  (params (ammo%20type :type AmmoList%20Enum :default "NewEnumerator0") (ammo%20size :type PickUpSizeEnum%20Enum :default "NewEnumerator0"))
  ;[0.15 0.15 0.15 0.5] add ammo
  (switch Utilities|FlowControl|Switch|SwitchonAmmoList ammo%20type
    (:NewEnumerator1
      (CallFunction|AddBullets ammo%20size))
    (:NewEnumerator2
      (CallFunction|Addrockets ammo%20size))))

(event Custom|add%20weapon
  (bind _weapontopickup (Variables|Default|GetweaponToPickup))
  (bind (_weaponname _weapon _amotype _ammosize) (Utilities|Struct|BreakSTWeaponData _weapontopickup))
  ;[0.15 0.15 0.15 0.5] add weapon
  (Utilities|Array|Add (Variables|Player|GetPlayerWeapons) _weapontopickup)
  (CallFunction|EquipWeapon _weapontopickup)
  (CallFunction|AddAmmo _amotype _ammosize))

(event EventBeginPlay
  ;[0.15 0.15 0.15 0.5] Init
  (|CallParentFunction)
  (bind _returnvalue (UserInterface|CreateWidget "/Game/FPS/Blueprints/Widgets/PlayerWeaponHUD.PlayerWeaponHUD_C"))
  (bind _output_get (Variables|Default|SetHUD _returnvalue))
  (UserInterface|Viewport|AddtoViewport _output_get 0)
  (Utilities|FlowControl|Delay 0.2)
  (CallFunction|UpdateUI)
  (CallFunction|InitWeapon "/Game/FPS/Blueprints/Player/PlayerWeaponBaseBP.PlayerWeaponBaseBP_C")
  (Default|Switchhweapon (Variables|Default|GetHUD) "NewEnumerator0"))

(event Collision|EventActorBeginOverlap
  (params (OtherActor :type Actor%20Object%20Reference)))

(event EventTick
  (params (DeltaSeconds :type Float%20%28single-precision%29))
  ;[0.15 0 0 0.5] weapon anim NOT USE
)

(event EventTakeDamage
  (params (Data :type Gameplay%20Cue%20Parameters%20Structure))
  ;[0.15 0.15 0.15 0.5] take Damage
  (|CallParentFunction Data)
  (CallFunction|UpdateUI)
  (bind _alpha (Timeline|DamageFlash PlayFromStart)
    (:Update
      (Default|SetFlashColor (Variables|Default|GetHUD) "(R=1.000000,G=0.079496,B=0.069946,A=1.000000)" _alpha))))

(event Input|ActionEvents|InputActionShoot
  (params (Key :type Key%20Structure :default "None"))
  ;[0.15 0.15 0.15 0.5] Fire Weapon
  (:Pressed
    (Abilities|TryActivateAbilitiesbyTag (Variables|Default|GetAbilitySystemComponent) (Variables|Default|GetweaponFireTag) false)))

(event Input|ActionEvents|InputActionSwitchPistol
  (params (Key :type Key%20Structure :default "None"))
  (:Pressed
    (if (CallFunction|HasWeapon "NewEnumerator1")
      (bind _weapondata (CallFunction|GetWeaponfromData "NewEnumerator1"))
      (CallFunction|EquipWeapon _weapondata))))

(event Input|ActionEvents|InputActionSwitchLauncher
  (params (Key :type Key%20Structure :default "None"))
  (:Pressed
    (if (CallFunction|HasWeapon "NewEnumerator2")
      (bind _weapondata (CallFunction|GetWeaponfromData "NewEnumerator2"))
      (CallFunction|EquipWeapon _weapondata))))

(event Input|AxisEvents|InputAxisLookHorizontal
  (params (AxisValue :type Float%20%28single-precision%29))
  ;[0.15 0.15 0.15 0.5] Move Camera
  (Pawn|Input|AddControllerYawInput AxisValue))

(event Input|AxisEvents|InputAxisLookVertical
  (params (AxisValue :type Float%20%28single-precision%29))
  ;[0.15 0.15 0.15 0.5] Move Camera
  (Pawn|Input|AddControllerPitchInput AxisValue))

(event Input|AxisEvents|InputAxisMoveHorizontal
  (params (AxisValue :type Float%20%28single-precision%29))
  ;[0.15 0.15 0.15 0.5] Player Movement
  (Pawn|Input|AddMovementInput (Math|Vector|GetForwardVector (Math|Rotator|MakeRotator 0.0 0.0 (.yaw (Pawn|GetControlRotation :!class /Script/Engine.Pawn)))) AxisValue false))

(event Input|AxisEvents|InputAxisMoveVertical
  (params (AxisValue :type Float%20%28single-precision%29))
  ;[0.15 0.15 0.15 0.5] Player Movement
  (Pawn|Input|AddMovementInput (Math|Vector|GetRightVector (Math|Rotator|MakeRotator 0.0 0.0 (.yaw (Pawn|GetControlRotation :!class /Script/Engine.Pawn)))) AxisValue false))

(fn ConstructionScript
  (|CallParentFunction))

(fn UpdateUI
  (bind _abilitysystemcomponent (Variables|Default|GetAbilitySystemComponent))
  (bind _hud (Variables|Default|GetHUD))
  (bind _hud_2 (Variables|Default|GetHUD))
  (bind _bulletstext (Variables|/Game/FPS/Blueprints/Widgets/PlayerWeaponHUD.PlayerWeaponHUD_C|GetBulletsText _hud_2))
  (Rendering|Components|TextRender|SetText (Variables|/Game/FPS/Blueprints/Widgets/PlayerWeaponHUD.PlayerWeaponHUD_C|GethealthText _hud) (Utilities|Text|ToText(Float) (.ReturnValue (Ability|Attribute|GetFloatAttributefromAbilitySystemComponent _abilitysystemcomponent "(AttributeName=\"Health\",Attribute=/Script/FPS.FPSAttributeSet:Health,AttributeOwner=\"/Script/CoreUObject.Class'/Script/FPS.FPSAttributeSet'\")")) "HalfToEven"))
  (Rendering|Components|TextRender|SetText (Variables|/Game/FPS/Blueprints/Widgets/PlayerWeaponHUD.PlayerWeaponHUD_C|GetArmorText _hud) (Utilities|Text|ToText(Float) (.ReturnValue (Ability|Attribute|GetFloatAttributefromAbilitySystemComponent _abilitysystemcomponent "(AttributeName=\"Armor\",Attribute=/Script/FPS.FPSAttributeSet:Armor,AttributeOwner=\"/Script/CoreUObject.Class'/Script/FPS.FPSAttributeSet'\")")) "HalfToEven"))
  (switch Utilities|FlowControl|Switch|SwitchonAmmoList (.amoType (Utilities|Struct|BreakSTWeaponData (Variables|Player|GetCurrentWeapon)))
    (:NewEnumerator1
      (Rendering|Components|TextRender|SetText _bulletstext (Utilities|Text|ToText(Float) (.ReturnValue (Ability|Attribute|GetFloatAttributefromAbilitySystemComponent (Variables|Default|GetAbilitySystemComponent) "(AttributeName=\"Bullets\",Attribute=/Script/FPS.FPSAttributeSet:Bullets,AttributeOwner=\"/Script/CoreUObject.Class'/Script/FPS.FPSAttributeSet'\")")) "HalfToEven")))
    (:NewEnumerator2
      (Rendering|Components|TextRender|SetText _bulletstext (Utilities|Text|ToText(Float) (.ReturnValue (Ability|Attribute|GetFloatAttributefromAbilitySystemComponent (Variables|Default|GetAbilitySystemComponent) "(AttributeName=\"Rockets\",Attribute=/Script/FPS.FPSAttributeSet:Rockets,AttributeOwner=\"/Script/CoreUObject.Class'/Script/FPS.FPSAttributeSet'\")")) "HalfToEven")))))

(fn HasWeapon
  (params (STWeaponData :type WeaponEnum%20Enum :default "NewEnumerator0"))
  (bind _array_element (Utilities|Array|ForEachLoopwithBreak (Variables|Player|GetPlayerWeapons) :!label _label)
    (:LoopBody
      (if (Utilities|Enum|Equal(Enum) (.weaponName (Utilities|Struct|BreakSTWeaponData _array_element)) STWeaponData)
        (LocalVariables|SetcompletedSearch true)
        (goto _label Break)))
    (:Completed
      (return (LocalVariables|GetcompletedSearch)))))

(fn GetWeaponfromData
  (params (weapon :type WeaponEnum%20Enum :default "NewEnumerator0"))
  (bind _outrownames (DataTable|GetDataTableRowNames "/Game/FPS/Blueprints/Weapon/DTWeapons.DTWeapons"))
  (bind _array_element (Utilities|Array|ForEachLoopwithBreak _outrownames :!label _label)
    (:LoopBody
      (bind _returnvalue (Utilities|GetDataTableRow "/Game/FPS/Blueprints/Weapon/DTWeapons.DTWeapons" _array_element)
        (:then
          (if (Utilities|Enum|Equal(Enum) weapon (.weaponName (Utilities|Struct|BreakSTWeaponData _returnvalue)))
            (LocalVariables|SetweaponExist true)
            (LocalVariables|SetweaponToEquip _returnvalue)
            (goto _label Break)))))
    (:Completed
      (return (LocalVariables|GetweaponToEquip) (LocalVariables|GetweaponExist)))))

(fn AddBullets
  (params (ammo%20size :type PickUpSizeEnum%20Enum :default "NewEnumerator0"))
  (if (not (>= (.ReturnValue (Ability|Attribute|GetFloatAttributefromAbilitySystemComponent (Variables|Default|GetAbilitySystemComponent) "(AttributeName=\"Bullets\",Attribute=/Script/FPS.FPSAttributeSet:Bullets,AttributeOwner=\"/Script/CoreUObject.Class'/Script/FPS.FPSAttributeSet'\")")) (Variables|Default|GetmaxBullets)))
    (switch Utilities|FlowControl|Switch|SwitchonPickUpSizeEnum ammo%20size
      (:NewEnumerator0
        (Variables|Default|SetammoTagContainer "(GameplayTags=((TagName=\"Pickup.Ammo.Bullets.Small\")))")
        (Abilities|TryActivateAbilitiesbyTag (Variables|Default|GetAbilitySystemComponent) (Variables|Default|GetammoTagContainer) true)
        (CallFunction|ItemPickup)))))

(fn InitWeapon
  (params (in%20Class :type Player%20Weapon%20Base%20BP%20Class%20Reference))
  (bind _weapon (Variables|Default|GetWeapon))
  (bind _childactor (Variables|/Script/Engine.ChildActorComponent|GetChildActor _weapon))
  (ChildActorComponent|SetChildActorClass _weapon in%20Class)
  (if (Utilities|DoesObjectImplementInterface _childactor "/Game/FPS/Blueprints/Interface/WeaponInterface.WeaponInterface_C")
    (Class|WeaponInterface|InitializeWeapon(Message) _childactor))
  (return _childactor))

(fn Addrockets
  (params (ammo%20size :type PickUpSizeEnum%20Enum :default "NewEnumerator0"))
  (if (not (>= (.ReturnValue (Ability|Attribute|GetFloatAttributefromAbilitySystemComponent (Variables|Default|GetAbilitySystemComponent) "(AttributeName=\"Rockets\",Attribute=/Script/FPS.FPSAttributeSet:Rockets,AttributeOwner=\"/Script/CoreUObject.Class'/Script/FPS.FPSAttributeSet'\")")) (Variables|Default|GetmaxRockets)))
    (switch Utilities|FlowControl|Switch|SwitchonPickUpSizeEnum ammo%20size
      (:NewEnumerator0
        (Variables|Default|SetammoTagContainer "(GameplayTags=((TagName=\"Pickup.Ammo.Rockets.Small\")))")
        (Abilities|TryActivateAbilitiesbyTag (Variables|Default|GetAbilitySystemComponent) (Variables|Default|GetammoTagContainer) true)
        (CallFunction|ItemPickup)))))