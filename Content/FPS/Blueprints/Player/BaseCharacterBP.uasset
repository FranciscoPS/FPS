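; Base character Blueprint in the FPS player folder that handles damage and death through the Gameplay Ability System.
; TakeDamage prints health and armor, then reports a damage event for AI sensing with the effect context's instigator and hit location.
; HealthCheck reads an ability system attribute and triggers KillCharacter at zero or below.
; KillCharacter is empty here, apparently a hook for child classes.
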(event Custom|TakeDamage
  (params (Data :type Gameplay%20Cue%20Parameters%20Structure))
  (bind (_normalizedmagnitude _rawmagnitude _effectcontext _matchedtagname _originaltag _aggregatedsourcetags _aggregatedtargettags _location) (Ability|GameplayCue|BreakGameplayCueParameters Data))
  (bind _abilitysystemcomponent (Variables|Default|GetAbilitySystemComponent))
  (Development|PrintString (Utilities|String|Append (Utilities|GetDisplayName self) "has health of " (Utilities|String|ToString(Float) (.ReturnValue (Ability|Attribute|GetFloatAttributefromAbilitySystemComponent _abilitysystemcomponent "(AttributeName=\"Health\",Attribute=/Script/FPS.FPSAttributeSet:Health,AttributeOwner=\"/Script/CoreUObject.Class'/Script/FPS.FPSAttributeSet'\")"))) ", has harmor of " (Utilities|String|ToString(Float) (.ReturnValue (Ability|Attribute|GetFloatAttributefromAbilitySystemComponent _abilitysystemcomponent "(AttributeName=\"Armor\",Attribute=/Script/FPS.FPSAttributeSet:Armor,AttributeOwner=\"/Script/CoreUObject.Class'/Script/FPS.FPSAttributeSet'\")")))))
  (Class|AISenseDamage|ReportDamageEvent self (Class|AbilitySystemBlueprintLibrary|EffectContextGetInstigatorActor _effectcontext) 0.0 _location "0, 0, 0" "None")
  (if (CallFunction|HealthCheck)
    (CallFunction|KillCharacter)))

(event Custom|KillCharacter)

(event EventBeginPlay)

(event Collision|EventActorBeginOverlap
  (params (OtherActor :type Actor%20Object%20Reference)))

(event EventTick
  (params (DeltaSeconds :type Float%20%28single-precision%29)))

(fn ConstructionScript)

(fn HealthCheck
  (return (<= (.ReturnValue (Ability|Attribute|GetFloatAttributefromAbilitySystemComponent (Variables|Default|GetAbilitySystemComponent) "(AttributeName=\"Health\",Attribute=/Script/FPS.FPSAttributeSet:Health,AttributeOwner=\"/Script/CoreUObject.Class'/Script/FPS.FPSAttributeSet'\")")) 0.0)))