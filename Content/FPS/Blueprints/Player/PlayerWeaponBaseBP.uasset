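; Base Blueprint for a first-person player weapon, drawn as a Paper2D flipbook.
; On BeginPlay it restricts a SceneCapture2D to render only the flipbook and stores the flipbook's rest position.
; InitializeWeapon resets the flipbook and hides it in game.
; WeaponMove plays the WalkAnim sequence while moving; otherwise it stops it and interpolates the flipbook back toward rest.
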(event Custom|WeaponMove
  (params (IsMoving :type Boolean) (Deltatime :type Float%20%28double-precision%29))
  (bind _walkanim (Variables|Default|GetWalkAnim))
  (bind _paperflipbook (Variables|Default|GetPaperFlipbook))
  (bind _sequenceplayer (Variables|/Script/ActorSequence.ActorSequenceComponent|GetSequencePlayer _walkanim))
  (if IsMoving
    (Sequencer|Player|Play _sequenceplayer :!class /Script/MovieScene.MovieSceneSequencePlayer)
    (else
      (Sequencer|Player|Stop _sequenceplayer :!class /Script/MovieScene.MovieSceneSequencePlayer)
      (Transformation|SetRelativeLocation _paperflipbook (Math|Interpolation|VInterpTo (Variables|/Script/Engine.SceneComponent|GetRelativeLocation _paperflipbook) (Variables|Default|GetWeaponPosition) Deltatime 0.0) false false))))

(event EventBeginPlay
  ;[0.15 0.15 0.15 0.5] SetRenderView
  (Rendering|SceneCapture|ShowOnlyComponent (Variables|Default|GetSceneCaptureComponent2D) (Variables|Default|GetPaperFlipbook))
  (Variables|Default|SetWeaponPosition (Variables|/Script/Engine.SceneComponent|GetRelativeLocation (Variables|Default|GetPaperFlipbook))))

(event Collision|EventActorBeginOverlap
  (params (OtherActor :type Actor%20Object%20Reference)))

(event EventTick
  (params (DeltaSeconds :type Float%20%28single-precision%29)))

(event EventInitializeWeapon
  (bind _paperflipbook (Variables|Default|GetPaperFlipbook))
  ;[0.15 0.15 0.15 0.5] InitNewWeapon
  (Sprite|SetFlipbook _paperflipbook)
  (Development|SetHiddeninGame _paperflipbook true false))

(fn ConstructionScript)