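; Base enemy Blueprint that renders as a billboarded Paper2D flipbook with directional walk and idle animations.
; Each tick it yaws the sprite toward the player camera, then computes the player's angle and side relative to its facing using 2D dot products.
; SetFace maps five facings plus left/right side to flipbooks, chosen by IsWalking.
; Tick currently always passes Front, so the computed angle does not yet select the facing.
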(event EventBeginPlay
  (|CallParentFunction) ; This node is disabled and will not be called.\nDrag off pins to build functionality.
)

(event Collision|EventActorBeginOverlap
  (params (OtherActor :type Actor%20Object%20Reference))
  (|CallParentFunction OtherActor) ; This node is disabled and will not be called.\nDrag off pins to build functionality.
)

(event EventTick
  (params (DeltaSeconds :type Float%20%28single-precision%29))
  (|CallParentFunction DeltaSeconds)
  (Utilities|SpriteFacePlayer
    (:Out
      (Utilities|GetEnemyAngle
        (:Out
          (Utilities|SetFace "NewEnumerator0"))))))

(fn ConstructionScript
  (|CallParentFunction))

(fn SetFlipbook
  (params (Walk :type Paper%20Flipbook%20Object%20Reference) (idle :type Paper%20Flipbook%20Object%20Reference))
  (bind _paperflipbook (Variables|Default|GetPaperFlipbook))
  (if (Variables|Default|GetIsWalking)
    (Sprite|SetFlipbook _paperflipbook Walk)
    (else
      (Sprite|SetFlipbook _paperflipbook idle))))